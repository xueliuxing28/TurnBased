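; BP_Pawn is a player camera pawn with smooth movement, stepped rotation and spring-arm zoom.
; Input axes shift a desired location along the actor's forward and right vectors and adjust a clamped desired zoom, while left and right actions rotate the desired rotation in 45-degree steps.
; Tick interpolates arm length, location and rotation toward these targets, which BeginPlay seeds from the starting state, without sweeping for collision.
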(event EventTick
  (params (DeltaSeconds :type Float%20%28single-precision%29))
  (bind _springarm (Variables|Default|GetSpringArm))
  (Variables|/Script/Engine.SpringArmComponent|SetTargetArmLength _springarm (Math|Interpolation|FInterpTo (Variables|/Script/Engine.SpringArmComponent|GetTargetArmLength _springarm) (Variables|Default|GetZoomDesired) DeltaSeconds 2.0))
  (Transformation|SetActorLocation (Math|Interpolation|VInterpTo (Transformation|GetActorLocation) (Variables|Default|GetLocationDesired) DeltaSeconds 3.0) false false)
  (Transformation|SetActorRotation (Math|Interpolation|RInterpTo (Transformation|GetActorRotation) (Variables|Default|GetRotationDesired) DeltaSeconds 3.0)))

(event EventBeginPlay
  (Variables|Default|SetZoomDesired (Variables|/Script/Engine.SpringArmComponent|GetTargetArmLength (Variables|Default|GetSpringArm)))
  (Variables|Default|SetLocationDesired (Transformation|GetActorLocation))
  (Variables|Default|SetRotationDesired (Transformation|GetActorRotation)))

(event Input|ActionEvents|InputActionRotationRight
  (params (Key :type Key%20Structure :default "None"))
  ;[0.1514 0.1329 1] 摄像机旋转
  (:Pressed
    (Variables|Default|SetRotationDesired (Math|Rotator|CombineRotators (Variables|Default|GetRotationDesired) "0,-45.000000, 0"))))

(event Input|ActionEvents|InputActionRotationLeft
  (params (Key :type Key%20Structure :default "None"))
  ;[0.1514 0.1329 1] 摄像机旋转
  (:Pressed
    (Variables|Default|SetRotationDesired (Math|Rotator|CombineRotators (Variables|Default|GetRotationDesired) "0,45.000000, 0"))))

(event Input|AxisEvents|InputAxisZoom
  (params (AxisValue :type Float%20%28single-precision%29))
  ;[0 1 0.7862] 摄像机缩放
  (Variables|Default|SetZoomDesired (Math|Float|Clamp(Float) (+ (Variables|Default|GetZoomDesired) (* AxisValue 4e+01)) 1e+02 5e+03)))

(event Input|AxisEvents|InputAxisForward
  (params (AxisValue :type Float%20%28single-precision%29))
  ;[0.1896 1 0.4063] 摄像机前后左右移动
  (Variables|Default|SetLocationDesired (+ (Variables|Default|GetLocationDesired) (* (* AxisValue 2e+01) (Transformation|GetActorForwardVector)))))

(event Input|AxisEvents|InputAxisRight
  (params (AxisValue :type Float%20%28single-precision%29))
  ;[0.1896 1 0.4063] 摄像机前后左右移动
  (Variables|Default|SetLocationDesired (+ (Variables|Default|GetLocationDesired) (* (* AxisValue 2e+01) (Transformation|GetActorRightVector)))))

(fn ConstructionScript)